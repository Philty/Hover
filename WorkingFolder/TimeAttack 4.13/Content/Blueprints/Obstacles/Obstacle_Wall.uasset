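; Moving wall obstacle that travels back and forth along a configurable direction.
; Tick moves the actor along the normalized DirectionOfMovement at Speed, scaled by delta time, basing each step on WallMesh's world transform without sweep.
; A looping delay chain from BeginPlay negates the direction after DurationOfMovement, then waits one more second before restarting, while movement continues throughout.
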(event `self.ReceiveBeginPlay`
  ;[1 1 1] Changing the DirectionofMovement after 5 seconds
  (`KismetSystemLibrary.Delay` (`self.DurationOfMovement`) :!label _label)
  (set `self.DirectionOfMovement` (`KismetMathLibrary.NegateVector` (`self.DirectionOfMovement`)))
  (`KismetSystemLibrary.Delay` 1.0)
  (goto _label))

(event `self.ReceiveTick`
  (params (DeltaSeconds :type "Float (single-precision)"))
  ;[1 1 1] Get Input Data and translate it to the mesh transformation
  (`self.K2_SetActorTransform` (`KismetMathLibrary.MakeTransform` (+ (* (`KismetMathLibrary.Normal` (`self.DirectionOfMovement`)) (* (`GameplayStatics.GetWorldDeltaSeconds`) (`self.Speed`))) (.location (`SceneComponent.K2_GetComponentToWorld` (`self.WallMesh`)))) (.rotation (`SceneComponent.K2_GetComponentToWorld` (`self.WallMesh`))) (.scale (`SceneComponent.K2_GetComponentToWorld` (`self.WallMesh`))))))

(fn `UserConstructionScript`)