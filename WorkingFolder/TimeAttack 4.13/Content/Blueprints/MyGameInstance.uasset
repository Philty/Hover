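; Game instance for a bumper car game that stores the player count and sets up cars for up to four local players.
; CreatePlayers moves each controller's car to a start and applies that player's stored mesh, material and color choices, using DoOnce gates to chain players by count.
; ChoosePlayerStart claims NetworkPlayerStarts by tagging them "Taken".
; HUDScaleToRatio scales HUD offsets and size from viewport size against a 1280x720 reference.
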(fn `ChoosePlayerStart`
  (returns (SelectedPlayerStart :type "PlayerStart Object Reference") (FoundPlayerSTart :type Boolean))
  (bind _outactors (`GameplayStatics.GetAllActorsOfClass` "/Game/Blueprints/NetworkPlayerStart.NetworkPlayerStart_C"))
  (for _array_element _outactors
    (if (!= (`PlayerStart.PlayerStartTag` _array_element) "Taken")
      (`|ExecutionSequence`
        (:`then_0`
          (break))
        (:`then_1`
          (set `PlayerStart.PlayerStartTag` "Taken" _array_element))
        (:`then_2`
          (return _array_element true))))))

(fn `CreatePlayers`
  (switch `/Game/Blueprints/E_NumberOfPlayers` (`self.NumberOfPlayers`)
    (:`NewEnumerator3`
      (bind _asbumper_car (cast `/Game/Blueprints/Vehicles/BumperCar` (`Controller.K2_GetPawn` (`GameplayStatics.GetPlayerController` 0)) :!label _label))
      (bind _selectedplayerstart (`self.ChoosePlayerStart`))
      (`Actor.K2_SetActorLocation` _asbumper_car (`Actor.K2_GetActorLocation` _selectedplayerstart) false true)
      (`/Game/Blueprints/Vehicles/BumperCar.ChangeVehicleMesh` _asbumper_car (`KismetArrayLibrary.Array_Get` (`self.CarMesh`)) (`KismetArrayLibrary.Array_Get` (`self.BodyMaterial`)) (`KismetArrayLibrary.Array_Get` (`self.BodyColor`)) (`KismetArrayLibrary.Array_Get` (`self.RingMaterial`)) (`KismetArrayLibrary.Array_Get` (`self.RingColor`)) (`KismetArrayLibrary.Array_Get` (`self.BodyDetailColor`)) (`KismetArrayLibrary.Array_Get` (`self.DetailBrightness`)) (`KismetArrayLibrary.Array_Get` (`self.RingDetailColor`)) (`KismetArrayLibrary.Array_Get` (`self.DetailBrightnessRing`)))
      (`/Engine/EditorBlueprintResources/StandardMacros.DoOnce` true :!label _label_2
        (:`Completed`
          _)))
    (:`NewEnumerator0`
      (`|ExecutionSequence`
        (:`then_0`
          (goto _label_2 :!via `Reset`))
        (:`then_1`
          (goto _label))))
    (:`NewEnumerator1`
      (`|ExecutionSequence`
        (:`then_0`
          (goto _label))
        (:`then_1`
          (goto _label_3 :!via `Reset`))
        (:`then_2`
          _)))
    (:`NewEnumerator2`
      (`|ExecutionSequence`
        (:`then_0`
          (goto _label))
        (:`then_1`
          (goto _label_3 :!via `Reset`))
        (:`then_2`
          (goto _label_4 :!via `Reset`))
        (:`then_3`
          _))))
  (bind _asbumper_car_2 (cast `/Game/Blueprints/Vehicles/BumperCar` (`Controller.K2_GetPawn` (`GameplayStatics.GetPlayerController` 1))))
  (bind _selectedplayerstart_2 (`self.ChoosePlayerStart`))
  (`Actor.K2_SetActorLocation` _asbumper_car_2 (`Actor.K2_GetActorLocation` _selectedplayerstart_2) false true)
  (set `/Game/Blueprints/Vehicles/BumperCar.PlayerIndexCache` 1 _asbumper_car_2)
  (`/Game/Blueprints/Vehicles/BumperCar.ChangeVehicleMesh` _asbumper_car_2 (`KismetArrayLibrary.Array_Get` (`self.CarMesh`) 1) (`KismetArrayLibrary.Array_Get` (`self.BodyMaterial`) 1) (`KismetArrayLibrary.Array_Get` (`self.BodyColor`) 1) (`KismetArrayLibrary.Array_Get` (`self.RingMaterial`) 1) (`KismetArrayLibrary.Array_Get` (`self.RingColor`) 1) (`KismetArrayLibrary.Array_Get` (`self.BodyDetailColor`) 1) (`KismetArrayLibrary.Array_Get` (`self.DetailBrightness`) 1) (`KismetArrayLibrary.Array_Get` (`self.RingDetailColor`) 1) (`KismetArrayLibrary.Array_Get` (`self.DetailBrightnessRing`) 1))
  (`/Engine/EditorBlueprintResources/StandardMacros.DoOnce` true :!label _label_3
    (:`Completed`
      (bind _asbumper_car_3 (cast `/Game/Blueprints/Vehicles/BumperCar` (`Controller.K2_GetPawn` (`GameplayStatics.GetPlayerController` 2))))
      (bind _selectedplayerstart_3 (`self.ChoosePlayerStart`))
      (`Actor.K2_SetActorLocation` _asbumper_car_3 (`Actor.K2_GetActorLocation` _selectedplayerstart_3) false true)
      (set `/Game/Blueprints/Vehicles/BumperCar.PlayerIndexCache` 2 _asbumper_car_3)
      (`/Game/Blueprints/Vehicles/BumperCar.ChangeVehicleMesh` _asbumper_car_3 (`KismetArrayLibrary.Array_Get` (`self.CarMesh`) 2) (`KismetArrayLibrary.Array_Get` (`self.BodyMaterial`) 2) (`KismetArrayLibrary.Array_Get` (`self.BodyColor`) 2) (`KismetArrayLibrary.Array_Get` (`self.RingMaterial`) 2) (`KismetArrayLibrary.Array_Get` (`self.RingColor`) 2) (`KismetArrayLibrary.Array_Get` (`self.BodyDetailColor`) 2) (`KismetArrayLibrary.Array_Get` (`self.DetailBrightness`) 2) (`KismetArrayLibrary.Array_Get` (`self.RingDetailColor`) 2) (`KismetArrayLibrary.Array_Get` (`self.DetailBrightnessRing`) 2))
      (`/Engine/EditorBlueprintResources/StandardMacros.DoOnce` true :!label _label_4
        (:`Completed`
          (bind _asbumper_car_4 (cast `/Game/Blueprints/Vehicles/BumperCar` (`Controller.K2_GetPawn` (`GameplayStatics.GetPlayerController` 3))))
          (bind _selectedplayerstart_4 (`self.ChoosePlayerStart`))
          (`Actor.K2_SetActorLocation` _asbumper_car_4 (`Actor.K2_GetActorLocation` _selectedplayerstart_4) false true)
          (`/Game/Blueprints/Vehicles/BumperCar.ChangeVehicleMesh` _asbumper_car_4 (`KismetArrayLibrary.Array_Get` (`self.CarMesh`) 3) (`KismetArrayLibrary.Array_Get` (`self.BodyMaterial`) 3) (`KismetArrayLibrary.Array_Get` (`self.BodyColor`) 3) (`KismetArrayLibrary.Array_Get` (`self.RingMaterial`) 3) (`KismetArrayLibrary.Array_Get` (`self.RingColor`) 3) (`KismetArrayLibrary.Array_Get` (`self.BodyDetailColor`) 3) (`KismetArrayLibrary.Array_Get` (`self.DetailBrightness`) 3) (`KismetArrayLibrary.Array_Get` (`self.RingDetailColor`) 3) (`KismetArrayLibrary.Array_Get` (`self.DetailBrightnessRing`) 3))
          (set `/Game/Blueprints/Vehicles/BumperCar.PlayerIndexCache` 3 _asbumper_car_4))))))

(fn `HUDScaleToRatio`
  (params (OffsetX :type "Float (double-precision)") (OffsetY :type "Float (double-precision)") (Scale :type "Float (double-precision)"))
  (returns (PositionX :type "Float (double-precision)") (PositionY :type "Float (double-precision)") (OutScale :type "Float (double-precision)"))
  (bind _ratioy (`self.RatioY`))
  (bind (_x _y) (`KismetMathLibrary.BreakVector2D` (`self.ScreenDimensions`)))
  (bind _asbumper_car (cast `/Game/Blueprints/Vehicles/BumperCar` (`GameplayStatics.GetPlayerController` (`self.MenuUserIndex`)))
    (:`then`
      (bind (_sizex _sizey) (`PlayerController.GetViewportSize` (`GameplayStatics.GetPlayerController` (`/Game/Blueprints/Vehicles/BumperCar.PlayerIndexCache` _asbumper_car))))
      (set `self.ScreenDimensions` (`KismetMathLibrary.MakeVector2D` (`KismetMathLibrary.Conv_IntToDouble` _sizex) (`KismetMathLibrary.Conv_IntToDouble` _sizey)))
      (`|ExecutionSequence`
        (:`then_0`
          (set `self.RatioX` (/ _x 1280.0)))
        (:`then_1`
          (set `self.RatioY` (/ _y 720.0)))
        (:`then_2`
          (return (* (`self.RatioX`) OffsetX) (* _ratioy OffsetY) (* Scale _ratioy)))))
    (:`CastFailed`
      (return (* (`self.RatioX`) OffsetX) (* _ratioy OffsetY) (* Scale _ratioy)))))

(fn `SetNumberOfPlayers`
  (params (Number :type "Float (double-precision)"))
  (bind _returnvalue (`KismetMathLibrary.FTrunc` Number))
  (set `self.IntNumberOfPlayers` _returnvalue)
  (if (== _returnvalue 1)
    (set `self.NumberOfPlayers` "NewEnumerator3")
    (elif (== _returnvalue 2)
      (set `self.NumberOfPlayers` "NewEnumerator0")
      (elif (== _returnvalue 3)
        (set `self.NumberOfPlayers` "NewEnumerator1")
        (elif (== _returnvalue 4)
          (set `self.NumberOfPlayers` "NewEnumerator2"))))))