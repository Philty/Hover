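; Ball actor for a two-player bumper car game that tracks which player touched it last.
; On hit by a BumperCar, it stores that car's player index and controller.
; Tick pushes the ball mesh's world location to both players' cars.
; DrawWinningHUD writes the last toucher's win message to their MyPlayerController and shows the HUDEndgame widget, with no caller in this graph.
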(event `self.ReceiveBeginPlay`)

(event `self.ReceiveHit`
  (params (MyComp :type "PrimitiveComponent Object Reference") (Other :type "Actor Object Reference") (OtherComp :type "PrimitiveComponent Object Reference") (bSelfMoved :type Boolean) (HitLocation :type "Vector Structure") (HitNormal :type "Vector Structure") (NormalImpulse :type "Vector Structure") (Hit :type "HitResult Structure (by ref)"))
  (bind _asbumper_car (cast `/Game/Blueprints/Vehicles/BumperCar` Other))
  (bind _playerindexcache (`/Game/Blueprints/Vehicles/BumperCar.PlayerIndexCache` _asbumper_car))
  (set `self.TouchedLast` _playerindexcache)
  (set `self.ControllerReference` (`GameplayStatics.GetPlayerController` _playerindexcache)))

(event `self.ReceiveTick`
  (params (DeltaSeconds :type "Float (single-precision)"))
  (for _index (range 2)
    (bind _asbumper_car (cast `/Game/Blueprints/Vehicles/BumperCar` (`GameplayStatics.GetPlayerPawn` _index)))
    (set `/Game/Blueprints/Vehicles/BumperCar.BallLocation` (`SceneComponent.K2_GetComponentLocation` (`self.StaticMesh`)) _asbumper_car)))

(fn `DrawWinningHUD`
  (bind _asmy_player_controller (cast `/Game/Blueprints/MyPlayerController` (`self.ControllerReference`)))
  (set `/Game/Blueprints/MyPlayerController.WinningPlayer` (`|FormatText` "Player {playerindex} wins!" (`KismetTextLibrary.Conv_IntToText` (`self.TouchedLast`))) _asmy_player_controller)
  (bind _returnvalue (`|CreateWidget` "/Game/Blueprints/UI/HUDEndgame.HUDEndgame_C" _asmy_player_controller))
  (`UserWidget.AddToViewport` _returnvalue 0))

(fn `UserConstructionScript`)