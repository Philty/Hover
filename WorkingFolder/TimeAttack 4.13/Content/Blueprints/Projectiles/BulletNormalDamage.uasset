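; A standard-damage bullet projectile that hurts bumper cars it hits.
; On a hit with a BumperCar, it subtracts a fixed amount from the car's current health, calls the car's health update, then destroys itself.
; Hits on other actors are ignored, and a short timer started at BeginPlay destroys the bullet regardless.
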(event `self.ReceiveBeginPlay`
  (`KismetSystemLibrary.Delay` 3.0)
  (`self.K2_DestroyActor`))

(event `self.ReceiveActorBeginOverlap`
  (params (OtherActor :type "Actor Object Reference")))

(event `self.ReceiveHit`
  (params (MyComp :type "PrimitiveComponent Object Reference") (Other :type "Actor Object Reference") (OtherComp :type "PrimitiveComponent Object Reference") (bSelfMoved :type Boolean) (HitLocation :type "Vector Structure") (HitNormal :type "Vector Structure") (NormalImpulse :type "Vector Structure") (Hit :type "HitResult Structure (by ref)"))
  (bind _asbumper_car (cast `/Game/Blueprints/Vehicles/BumperCar` Other))
  (`self.DamagePlayer` _asbumper_car)
  (`self.K2_DestroyActor`))

(event `self.ReceiveTick`
  (params (DeltaSeconds :type "Float (single-precision)")))

(fn `DamagePlayer`
  (params (BumperCar :type "/Game/Blueprints/Vehicles/BumperCar Object Reference"))
  (set `/Game/Blueprints/Vehicles/BumperCar.CurrentHealth` (- (`/Game/Blueprints/Vehicles/BumperCar.CurrentHealth` BumperCar) 50.0) BumperCar)
  (`/Game/Blueprints/Vehicles/BumperCar.UpdateHealth` BumperCar))

(fn `UserConstructionScript`)