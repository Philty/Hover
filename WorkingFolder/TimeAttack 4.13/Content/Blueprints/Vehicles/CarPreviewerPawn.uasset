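; Pawn that previews a player's customizable drone vehicle and rotates it with input axes, with the gamepad top face button resetting rotation.
; Every tick it reads that player's mesh and material choices from MyGameInstance and passes them to ChangeVehicleMesh.
; That function swaps body, jet and ring meshes, then creates and tints per-drone dynamic material instances, with jet and ring sharing the ring material.
; Tick also calls JetAndRingRotation.
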(event `self.ReceiveBeginPlay`
  (bind _asmy_player_controller (cast `/Game/Blueprints/MyPlayerController` (`GameplayStatics.GetPlayerController` (`self.PlayerIndexCache`))))
  (set `self.ControllerReference` _asmy_player_controller))

(event `self.ReceiveTick`
  (params (DeltaSeconds :type "Float (single-precision)"))
  (bind _playerindexcache (`self.PlayerIndexCache`))
  (bind _asmy_game_instance (cast `/Game/Blueprints/MyGameInstance` (`GameplayStatics.GetGameInstance`)))
  (`self.ChangeVehicleMesh` (`KismetArrayLibrary.Array_Get` (`/Game/Blueprints/MyGameInstance.CarMesh` _asmy_game_instance) _playerindexcache) (`KismetArrayLibrary.Array_Get` (`/Game/Blueprints/MyGameInstance.BodyMaterial` _asmy_game_instance) _playerindexcache) (`KismetArrayLibrary.Array_Get` (`/Game/Blueprints/MyGameInstance.RingMaterial` _asmy_game_instance) _playerindexcache))
  (`self.K2_AddActorLocalRotation` (`KismetMathLibrary.MakeRotator` (* (`self.RotatingSpeed`) (`self.GetInputAxisKeyValue`)) (* (`self.GetInputAxisKeyValue`) (`self.RotatingSpeed`))))
  (`self.JetAndRingRotation`))

(event `Key|Gamepad_FaceButton_Top`
  (params (Key :type "Key Structure" :default "AnyKey"))
  (:`Pressed`
    (`self.ResetRotation`)))

(fn `ChangeVehicleMesh`
  (params (StaticMeshInteger :type Integer) (BodyMaterialNumber :type Integer) (RingMaterialNumber :type Integer))
  (bind _car (`self.Car`))
  (bind _carjet (`self.CarJet`))
  (bind _carjet_2 (`self.CarJet`))
  (bind _carjet_3 (`self.CarJet`))
  (bind _car_2 (`self.Car`))
  (bind _carjet_4 (`self.CarJet`))
  (bind _carring (`self.CarRing`))
  (bind _car_3 (`self.Car`))
  (bind _carring_2 (`self.CarRing`))
  (bind _car_4 (`self.Car`))
  (bind _carring_3 (`self.CarRing`))
  (bind _returnvalue (`KismetSystemLibrary.GetObjectName` (`StaticMeshComponent.StaticMesh` _car_3)))
  (`|ExecutionSequence`
    (:`then_0`
      (switch `int` StaticMeshInteger
        (:`0`
          (`StaticMeshComponent.SetStaticMesh` _car "/Game/Geometry/Vehicles/Drone1/Drone1.Drone1")
          (`StaticMeshComponent.SetStaticMesh` _carjet "/Game/Geometry/Vehicles/Drone1/Drone1Jet.Drone1Jet")
          (`StaticMeshComponent.SetStaticMesh` (`self.CarRing`) "/Game/Geometry/Vehicles/Drone1/Drone1Ring.Drone1Ring"))
        (:`1`
          (`StaticMeshComponent.SetStaticMesh` _car "/Game/Geometry/Vehicles/Drone2/Drone2.Drone2")
          (`StaticMeshComponent.SetStaticMesh` _carjet "/Game/Geometry/Vehicles/Drone2/Drone2Jet.Drone2Jet")
          (`StaticMeshComponent.SetStaticMesh` (`self.CarRing`) "/Game/Geometry/Vehicles/Drone2/Drone2Ring.Drone2Ring"))
        (:`2`
          (`StaticMeshComponent.SetStaticMesh` _car "/Game/Geometry/Vehicles/Drone3/Drone3.Drone3")
          (`StaticMeshComponent.SetStaticMesh` (`self.CarJet`) "/Game/Geometry/Vehicles/Drone3/Drone3Jet.Drone3Jet")
          (`StaticMeshComponent.SetStaticMesh` (`self.CarRing`) "/Game/Geometry/Vehicles/Drone3/Drone3Ring.Drone3Ring"))))
    (:`then_1`
      ;[1 1 1] Drone1
      (if (== _returnvalue "drone1")
        (`|ExecutionSequence`
          (:`then_0`
            (switch `int` BodyMaterialNumber
              (:`0`
                (bind _returnvalue_2 (`PrimitiveComponent.CreateDynamicMaterialInstance` _car_3 0 "/Game/Geometry/Vehicles/Drone1/M_Carpaint_Drone1_Inst.M_Carpaint_Drone1_Inst"))
                (`MaterialInstanceDynamic.SetVectorParameterValue` _returnvalue_2 "Base Color" (`self.BodyColor`))
                (`MaterialInstanceDynamic.SetVectorParameterValue` _returnvalue_2 "Flake Color" (`self.BodyDetailColor`))
                (`MaterialInstanceDynamic.SetScalarParameterValue` _returnvalue_2 "Flake Brightness" (`self.BodyDetailBrightness`)))
              (:`1`
                (bind _returnvalue_3 (`PrimitiveComponent.CreateDynamicMaterialInstance` _car_3 0 "/Game/Geometry/Vehicles/Drone1/M_Plastic_Coated_Drone1__Inst.M_Plastic_Coated_Drone1__Inst"))
                (`MaterialInstanceDynamic.SetVectorParameterValue` _returnvalue_3 "Base Color" (`self.BodyColor`)))
              (:`2`
                (bind _returnvalue_4 (`PrimitiveComponent.CreateDynamicMaterialInstance` _car_3 0 "/Game/Geometry/Vehicles/Drone1/M_Plastic_Matte_Drone1_Inst.M_Plastic_Matte_Drone1_Inst"))
                (`MaterialInstanceDynamic.SetVectorParameterValue` _returnvalue_4 "Base Color" (`self.BodyColor`)))
              (:`3`
                (bind _returnvalue_5 (`PrimitiveComponent.CreateDynamicMaterialInstance` _car_3 0 "/Game/Geometry/Vehicles/Drone1/M_Plastic_Speckled_Drone1_Inst.M_Plastic_Speckled_Drone1_Inst"))
                (`MaterialInstanceDynamic.SetVectorParameterValue` _returnvalue_5 "Base Color" (`self.BodyColor`))
                (`MaterialInstanceDynamic.SetVectorParameterValue` _returnvalue_5 "Flake Color" (`self.BodyDetailColor`))
                (`MaterialInstanceDynamic.SetScalarParameterValue` _returnvalue_5 "Flake Brightness" (`self.BodyDetailBrightness`)))
              (:`4`
                (bind _returnvalue_6 (`PrimitiveComponent.CreateDynamicMaterialInstance` _car_3 0 "/Game/Geometry/Vehicles/Drone1/M_CarbonFiber_Drone1_Inst.M_CarbonFiber_Drone1_Inst"))
                (`MaterialInstanceDynamic.SetVectorParameterValue` _returnvalue_6 "Base Color" (`self.BodyColor`)))
              (:`5`
                (bind _returnvalue_7 (`PrimitiveComponent.CreateDynamicMaterialInstance` _car_3 0 "/Game/Geometry/Vehicles/Drone1/M_TireRubber_Drone1_Inst.M_TireRubber_Drone1_Inst"))
                (`MaterialInstanceDynamic.SetVectorParameterValue` _returnvalue_7 "Base Color" (`self.BodyColor`)))
              (:`6`
                (bind _returnvalue_8 (`PrimitiveComponent.CreateDynamicMaterialInstance` _car_3 0 "/Game/Geometry/Vehicles/Drone1/M_Metal_Drone1_Inst.M_Metal_Drone1_Inst"))
                (`MaterialInstanceDynamic.SetVectorParameterValue` _returnvalue_8 "Base Color" (`self.BodyColor`)))
              (:`7`
                (bind _returnvalue_9 (`PrimitiveComponent.CreateDynamicMaterialInstance` _car_3 0 "/Game/Geometry/Vehicles/Drone1/M_Alcantara_Drone1_Inst.M_Alcantara_Drone1_Inst"))
                (`MaterialInstanceDynamic.SetVectorParameterValue` _returnvalue_9 "Base Color" (`self.BodyColor`))
                (`MaterialInstanceDynamic.SetVectorParameterValue` _returnvalue_9 "Rim Color" (`self.BodyDetailColor`)))
              (:`8`
                (bind _returnvalue_10 (`PrimitiveComponent.CreateDynamicMaterialInstance` _car_3 0 "/Game/Geometry/Vehicles/Drone1/M_Fabric_ArchLiner_Inst.M_Fabric_ArchLiner_Inst"))
                (`MaterialInstanceDynamic.SetVectorParameterValue` _returnvalue_10 "Base Color" (`self.BodyColor`)))
              (:`9`
                (bind _returnvalue_11 (`PrimitiveComponent.CreateDynamicMaterialInstance` _car_3 0 "/Game/Geometry/Vehicles/Drone1/M_Leather_Drone1_Inst.M_Leather_Drone1_Inst"))
                (`MaterialInstanceDynamic.SetVectorParameterValue` _returnvalue_11 "Base Color" (`self.BodyColor`)))
              (:`10`
                (bind _returnvalue_12 (`PrimitiveComponent.CreateDynamicMaterialInstance` _car_3 0 "/Game/Geometry/Vehicles/Drone1/MI_MasterPerforated_Drone1_Inst.MI_MasterPerforated_Drone1_Inst"))
                (`MaterialInstanceDynamic.SetVectorParameterValue` _returnvalue_12 "Base Color" (`self.BodyColor`))
                (`MaterialInstanceDynamic.SetVectorParameterValue` _returnvalue_12 "Perforation Color" (`self.BodyDetailColor`)))))
          (:`then_1`
            (switch `int` RingMaterialNumber
              (:`0`
                (bind _returnvalue_13 (`PrimitiveComponent.CreateDynamicMaterialInstance` _carjet_3 0 "/Game/Geometry/Vehicles/Drone1/M_Carpaint_Drone1_Inst.M_Carpaint_Drone1_Inst"))
                (`MaterialInstanceDynamic.SetVectorParameterValue` _returnvalue_13 "Base Color" (`self.RingColor`))
                (`MaterialInstanceDynamic.SetVectorParameterValue` _returnvalue_13 "Flake Color" (`self.RingDetailColor`))
                (`MaterialInstanceDynamic.SetScalarParameterValue` _returnvalue_13 "Flake Brightness" (`self.RingDetailBrightness`)))
              (:`1`
                (bind _returnvalue_14 (`PrimitiveComponent.CreateDynamicMaterialInstance` _carjet_3 0 "/Game/Geometry/Vehicles/Drone1/M_Plastic_Coated_Drone1__Inst.M_Plastic_Coated_Drone1__Inst"))
                (`MaterialInstanceDynamic.SetVectorParameterValue` _returnvalue_14 "Base Color" (`self.RingColor`)))
              (:`2`
                (bind _returnvalue_15 (`PrimitiveComponent.CreateDynamicMaterialInstance` _carjet_3 0 "/Game/Geometry/Vehicles/Drone1/M_Plastic_Matte_Drone1_Inst.M_Plastic_Matte_Drone1_Inst"))
                (`MaterialInstanceDynamic.SetVectorParameterValue` _returnvalue_15 "Base Color" (`self.RingColor`)))
              (:`3`
                (bind _returnvalue_16 (`PrimitiveComponent.CreateDynamicMaterialInstance` _carjet_3 0 "/Game/Geometry/Vehicles/Drone1/M_Plastic_Speckled_Drone1_Inst.M_Plastic_Speckled_Drone1_Inst"))
                (`MaterialInstanceDynamic.SetVectorParameterValue` _returnvalue_16 "Base Color" (`self.RingColor`))
                (`MaterialInstanceDynamic.SetVectorParameterValue` _returnvalue_16 "Flake Color" (`self.RingDetailColor`))
                (`MaterialInstanceDynamic.SetScalarParameterValue` _returnvalue_16 "Flake Brightness" (`self.RingDetailBrightness`)))
              (:`4`
                (bind _returnvalue_17 (`PrimitiveComponent.CreateDynamicMaterialInstance` _carjet_3 0 "/Game/Geometry/Vehicles/Drone1/M_CarbonFiber_Drone1_Inst.M_CarbonFiber_Drone1_Inst"))
                (`MaterialInstanceDynamic.SetVectorParameterValue` _returnvalue_17 "Base Color" (`self.RingColor`)))
              (:`5`
                (bind _returnvalue_18 (`PrimitiveComponent.CreateDynamicMaterialInstance` _carjet_3 0 "/Game/Geometry/Vehicles/Drone1/M_TireRubber_Drone1_Inst.M_TireRubber_Drone1_Inst"))
                (`MaterialInstanceDynamic.SetVectorParameterValue` _returnvalue_18 "Base Color" (`self.RingColor`)))
              (:`6`
                (bind _returnvalue_19 (`PrimitiveComponent.CreateDynamicMaterialInstance` _carjet_3 0 "/Game/Geometry/Vehicles/Drone1/M_Metal_Drone1_Inst.M_Metal_Drone1_Inst"))
                (`MaterialInstanceDynamic.SetVectorParameterValue` _returnvalue_19 "Base Color" (`self.RingColor`)))
              (:`7`
                (bind _returnvalue_20 (`PrimitiveComponent.CreateDynamicMaterialInstance` _carjet_3 0 "/Game/Geometry/Vehicles/Drone1/M_Alcantara_Drone1_Inst.M_Alcantara_Drone1_Inst"))
                (`MaterialInstanceDynamic.SetVectorParameterValue` _returnvalue_20 "Base Color" (`self.RingColor`))
                (`MaterialInstanceDynamic.SetVectorParameterValue` _returnvalue_20 "Rim Color" (`self.RingDetailColor`)))
              (:`8`
                (bind _returnvalue_21 (`PrimitiveComponent.CreateDynamicMaterialInstance` _carjet_3 0 "/Game/Geometry/Vehicles/Drone1/M_Fabric_ArchLiner_Inst.M_Fabric_ArchLiner_Inst"))
                (`MaterialInstanceDynamic.SetVectorParameterValue` _returnvalue_21 "Base Color" (`self.RingColor`)))
              (:`9`
                (bind _returnvalue_22 (`PrimitiveComponent.CreateDynamicMaterialInstance` _carjet_3 0 "/Game/Geometry/Vehicles/Drone1/M_Leather_Drone1_Inst.M_Leather_Drone1_Inst"))
                (`MaterialInstanceDynamic.SetVectorParameterValue` _returnvalue_22 "Base Color" (`self.RingColor`)))
              (:`10`
                (bind _returnvalue_23 (`PrimitiveComponent.CreateDynamicMaterialInstance` _carjet_3 0 "/Game/Geometry/Vehicles/Drone1/MI_MasterPerforated_Drone1_Inst.MI_MasterPerforated_Drone1_Inst"))
                (`MaterialInstanceDynamic.SetVectorParameterValue` _returnvalue_23 "Base Color" (`self.RingColor`))
                (`MaterialInstanceDynamic.SetVectorParameterValue` _returnvalue_23 "Perforation Color" (`self.RingDetailColor`)))))
          (:`then_2`
            (switch `int` RingMaterialNumber
              (:`0`
                (bind _returnvalue_24 (`PrimitiveComponent.CreateDynamicMaterialInstance` _carring_2 0 "/Game/Geometry/Vehicles/Drone1/M_Carpaint_Drone1_Inst.M_Carpaint_Drone1_Inst"))
                (`MaterialInstanceDynamic.SetVectorParameterValue` _returnvalue_24 "Base Color" (`self.RingColor`))
                (`MaterialInstanceDynamic.SetVectorParameterValue` _returnvalue_24 "Flake Color" (`self.RingDetailColor`))
                (`MaterialInstanceDynamic.SetScalarParameterValue` _returnvalue_24 "Flake Brightness" (`self.RingDetailBrightness`)))
              (:`1`
                (bind _returnvalue_25 (`PrimitiveComponent.CreateDynamicMaterialInstance` _carring_2 0 "/Game/Geometry/Vehicles/Drone1/M_Plastic_Coated_Drone1__Inst.M_Plastic_Coated_Drone1__Inst"))
                (`MaterialInstanceDynamic.SetVectorParameterValue` _returnvalue_25 "Base Color" (`self.RingColor`)))
              (:`2`
                (bind _returnvalue_26 (`PrimitiveComponent.CreateDynamicMaterialInstance` _carring_2 0 "/Game/Geometry/Vehicles/Drone1/M_Plastic_Matte_Drone1_Inst.M_Plastic_Matte_Drone1_Inst"))
                (`MaterialInstanceDynamic.SetVectorParameterValue` _returnvalue_26 "Base Color" (`self.RingColor`)))
              (:`3`
                (bind _returnvalue_27 (`PrimitiveComponent.CreateDynamicMaterialInstance` _carring_2 0 "/Game/Geometry/Vehicles/Drone1/M_Plastic_Speckled_Drone1_Inst.M_Plastic_Speckled_Drone1_Inst"))
                (`MaterialInstanceDynamic.SetVectorParameterValue` _returnvalue_27 "Base Color" (`self.RingColor`))
                (`MaterialInstanceDynamic.SetVectorParameterValue` _returnvalue_27 "Flake Color" (`self.RingDetailColor`))
                (`MaterialInstanceDynamic.SetScalarParameterValue` _returnvalue_27 "Flake Brightness" (`self.RingDetailBrightness`)))
              (:`4`
                (bind _returnvalue_28 (`PrimitiveComponent.CreateDynamicMaterialInstance` _carring_2 0 "/Game/Geometry/Vehicles/Drone1/M_CarbonFiber_Drone1_Inst.M_CarbonFiber_Drone1_Inst"))
                (`MaterialInstanceDynamic.SetVectorParameterValue` _returnvalue_28 "Base Color" (`self.RingColor`)))
              (:`5`
                (bind _returnvalue_29 (`PrimitiveComponent.CreateDynamicMaterialInstance` _carring_2 0 "/Game/Geometry/Vehicles/Drone1/M_TireRubber_Drone1_Inst.M_TireRubber_Drone1_Inst"))
                (`MaterialInstanceDynamic.SetVectorParameterValue` _returnvalue_29 "Base Color" (`self.RingColor`)))
              (:`6`
                (bind _returnvalue_30 (`PrimitiveComponent.CreateDynamicMaterialInstance` _carring_2 0 "/Game/Geometry/Vehicles/Drone1/M_Metal_Drone1_Inst.M_Metal_Drone1_Inst"))
                (`MaterialInstanceDynamic.SetVectorParameterValue` _returnvalue_30 "Base Color" (`self.RingColor`)))
              (:`7`
                (bind _returnvalue_31 (`PrimitiveComponent.CreateDynamicMaterialInstance` _carring_2 0 "/Game/Geometry/Vehicles/Drone1/M_Alcantara_Drone1_Inst.M_Alcantara_Drone1_Inst"))
                (`MaterialInstanceDynamic.SetVectorParameterValue` _returnvalue_31 "Base Color" (`self.RingColor`))
                (`MaterialInstanceDynamic.SetVectorParameterValue` _returnvalue_31 "Rim Color" (`self.RingDetailColor`)))
              (:`8`
                (bind _returnvalue_32 (`PrimitiveComponent.CreateDynamicMaterialInstance` _carring_2 0 "/Game/Geometry/Vehicles/Drone1/M_Fabric_ArchLiner_Inst.M_Fabric_ArchLiner_Inst"))
                (`MaterialInstanceDynamic.SetVectorParameterValue` _returnvalue_32 "Base Color" (`self.RingColor`)))
              (:`9`
                (bind _returnvalue_33 (`PrimitiveComponent.CreateDynamicMaterialInstance` _carring_2 0 "/Game/Geometry/Vehicles/Drone1/M_Leather_Drone1_Inst.M_Leather_Drone1_Inst"))
                (`MaterialInstanceDynamic.SetVectorParameterValue` _returnvalue_33 "Base Color" (`self.RingColor`)))
              (:`10`
                (bind _returnvalue_34 (`PrimitiveComponent.CreateDynamicMaterialInstance` _carring_2 0 "/Game/Geometry/Vehicles/Drone1/MI_MasterPerforated_Drone1_Inst.MI_MasterPerforated_Drone1_Inst"))
                (`MaterialInstanceDynamic.SetVectorParameterValue` _returnvalue_34 "Base Color" (`self.RingColor`))
                (`MaterialInstanceDynamic.SetVectorParameterValue` _returnvalue_34 "Perforation Color" (`self.RingDetailColor`))))))
        (else
          ;[1 1 1] Drone2
          (if (== _returnvalue "drone2")
            (`|ExecutionSequence`
              (:`then_0`
                (switch `int` BodyMaterialNumber
                  (:`0`
                    (bind _returnvalue_35 (`PrimitiveComponent.CreateDynamicMaterialInstance` _car_2 0 "/Game/Geometry/Vehicles/Drone2/M_Carpaint_Drone2_Inst.M_Carpaint_Drone2_Inst"))
                    (`MaterialInstanceDynamic.SetVectorParameterValue` _returnvalue_35 "Base Color" (`self.BodyColor`))
                    (`MaterialInstanceDynamic.SetVectorParameterValue` _returnvalue_35 "Flake Color" (`self.BodyDetailColor`))
                    (`MaterialInstanceDynamic.SetScalarParameterValue` _returnvalue_35 "Flake Brightness" (`self.BodyDetailBrightness`)))
                  (:`1`
                    (bind _returnvalue_36 (`PrimitiveComponent.CreateDynamicMaterialInstance` _car_2 0 "/Game/Geometry/Vehicles/Drone2/M_Plastic_Coated_Drone2_Inst.M_Plastic_Coated_Drone2_Inst"))
                    (`MaterialInstanceDynamic.SetVectorParameterValue` _returnvalue_36 "Base Color" (`self.BodyColor`)))
                  (:`2`
                    (bind _returnvalue_37 (`PrimitiveComponent.CreateDynamicMaterialInstance` _car_2 0 "/Game/Geometry/Vehicles/Drone2/M_Plastic_Matte_Drone2_Inst.M_Plastic_Matte_Drone2_Inst"))
                    (`MaterialInstanceDynamic.SetVectorParameterValue` _returnvalue_37 "Base Color" (`self.BodyColor`)))
                  (:`3`
                    (bind _returnvalue_38 (`PrimitiveComponent.CreateDynamicMaterialInstance` _car_2 0 "/Game/Geometry/Vehicles/Drone2/M_Plastic_Speckled_Drone2_Inst.M_Plastic_Speckled_Drone2_Inst"))
                    (`MaterialInstanceDynamic.SetVectorParameterValue` _returnvalue_38 "Base Color" (`self.BodyColor`))
                    (`MaterialInstanceDynamic.SetVectorParameterValue` _returnvalue_38 "Flake Color" (`self.BodyDetailColor`))
                    (`MaterialInstanceDynamic.SetScalarParameterValue` _returnvalue_38 "Flake Brightness" (`self.BodyDetailBrightness`)))
                  (:`4`
                    (bind _returnvalue_39 (`PrimitiveComponent.CreateDynamicMaterialInstance` _car_2 0 "/Game/Geometry/Vehicles/Drone2/M_CarbonFiber_Drone2_Inst.M_CarbonFiber_Drone2_Inst"))
                    (`MaterialInstanceDynamic.SetVectorParameterValue` _returnvalue_39 "Base Color" (`self.BodyColor`)))
                  (:`5`
                    (bind _returnvalue_40 (`PrimitiveComponent.CreateDynamicMaterialInstance` _car_2 0 "/Game/Geometry/Vehicles/Drone2/M_TireRubber_Drone2_Inst.M_TireRubber_Drone2_Inst"))
                    (`MaterialInstanceDynamic.SetVectorParameterValue` _returnvalue_40 "Base Color" (`self.BodyColor`)))
                  (:`6`
                    (bind _returnvalue_41 (`PrimitiveComponent.CreateDynamicMaterialInstance` _car_2 0 "/Game/Geometry/Vehicles/Drone2/M_Metal_Drone2_Inst.M_Metal_Drone2_Inst"))
                    (`MaterialInstanceDynamic.SetVectorParameterValue` _returnvalue_41 "Base Color" (`self.BodyColor`)))
                  (:`7`
                    (bind _returnvalue_42 (`PrimitiveComponent.CreateDynamicMaterialInstance` _car_2 0 "/Game/Geometry/Vehicles/Drone2/M_Alcantara_Drone2_Inst.M_Alcantara_Drone2_Inst"))
                    (`MaterialInstanceDynamic.SetVectorParameterValue` _returnvalue_42 "Base Color" (`self.BodyColor`))
                    (`MaterialInstanceDynamic.SetVectorParameterValue` _returnvalue_42 "Rim Color" (`self.BodyDetailColor`)))
                  (:`8`
                    (bind _returnvalue_43 (`PrimitiveComponent.CreateDynamicMaterialInstance` _car_2 0 "/Game/Geometry/Vehicles/Drone2/M_Fabric_ArchLiner_Drone2_Inst.M_Fabric_ArchLiner_Drone2_Inst"))
                    (`MaterialInstanceDynamic.SetVectorParameterValue` _returnvalue_43 "Base Color" (`self.BodyColor`)))
                  (:`9`
                    (bind _returnvalue_44 (`PrimitiveComponent.CreateDynamicMaterialInstance` _car_2 0 "/Game/Geometry/Vehicles/Drone2/M_Leather_Drone2_Inst.M_Leather_Drone2_Inst"))
                    (`MaterialInstanceDynamic.SetVectorParameterValue` _returnvalue_44 "Base Color" (`self.BodyColor`)))
                  (:`10`
                    (bind _returnvalue_45 (`PrimitiveComponent.CreateDynamicMaterialInstance` _car_2 0 "/Game/Geometry/Vehicles/Drone2/MI_MasterPerforated_Drone2_Inst.MI_MasterPerforated_Drone2_Inst"))
                    (`MaterialInstanceDynamic.SetVectorParameterValue` _returnvalue_45 "Base Color" (`self.BodyColor`))
                    (`MaterialInstanceDynamic.SetVectorParameterValue` _returnvalue_45 "Perforation Color" (`self.BodyDetailColor`)))))
              (:`then_1`
                (switch `int` RingMaterialNumber
                  (:`0`
                    (bind _returnvalue_46 (`PrimitiveComponent.CreateDynamicMaterialInstance` _carjet_4 0 "/Game/Geometry/Vehicles/Drone2/M_Carpaint_Drone2_Inst.M_Carpaint_Drone2_Inst"))
                    (`MaterialInstanceDynamic.SetVectorParameterValue` _returnvalue_46 "Base Color" (`self.RingColor`))
                    (`MaterialInstanceDynamic.SetVectorParameterValue` _returnvalue_46 "Flake Color" (`self.RingDetailColor`))
                    (`MaterialInstanceDynamic.SetScalarParameterValue` _returnvalue_46 "Flake Brightness" (`self.RingDetailBrightness`)))
                  (:`1`
                    (bind _returnvalue_47 (`PrimitiveComponent.CreateDynamicMaterialInstance` _carjet_4 0 "/Game/Geometry/Vehicles/Drone2/M_Plastic_Coated_Drone2_Inst.M_Plastic_Coated_Drone2_Inst"))
                    (`MaterialInstanceDynamic.SetVectorParameterValue` _returnvalue_47 "Base Color" (`self.RingColor`)))
                  (:`2`
                    (bind _returnvalue_48 (`PrimitiveComponent.CreateDynamicMaterialInstance` _carjet_4 0 "/Game/Geometry/Vehicles/Drone2/M_Plastic_Matte_Drone2_Inst.M_Plastic_Matte_Drone2_Inst"))
                    (`MaterialInstanceDynamic.SetVectorParameterValue` _returnvalue_48 "Base Color" (`self.RingColor`)))
                  (:`3`
                    (bind _returnvalue_49 (`PrimitiveComponent.CreateDynamicMaterialInstance` _carjet_4 0 "/Game/Geometry/Vehicles/Drone2/M_Plastic_Speckled_Drone2_Inst.M_Plastic_Speckled_Drone2_Inst"))
                    (`MaterialInstanceDynamic.SetVectorParameterValue` _returnvalue_49 "Base Color" (`self.RingColor`))
                    (`MaterialInstanceDynamic.SetVectorParameterValue` _returnvalue_49 "Flake Color" (`self.RingDetailColor`))
                    (`MaterialInstanceDynamic.SetScalarParameterValue` _returnvalue_49 "Flake Brightness" (`self.RingDetailBrightness`)))
                  (:`4`
                    (bind _returnvalue_50 (`PrimitiveComponent.CreateDynamicMaterialInstance` _carjet_4 0 "/Game/Geometry/Vehicles/Drone2/M_CarbonFiber_Drone2_Inst.M_CarbonFiber_Drone2_Inst"))
                    (`MaterialInstanceDynamic.SetVectorParameterValue` _returnvalue_50 "Base Color" (`self.RingColor`)))
                  (:`5`
                    (bind _returnvalue_51 (`PrimitiveComponent.CreateDynamicMaterialInstance` _carjet_4 0 "/Game/Geometry/Vehicles/Drone2/M_TireRubber_Drone2_Inst.M_TireRubber_Drone2_Inst"))
                    (`MaterialInstanceDynamic.SetVectorParameterValue` _returnvalue_51 "Base Color" (`self.RingColor`)))
                  (:`6`
                    (bind _returnvalue_52 (`PrimitiveComponent.CreateDynamicMaterialInstance` _carjet_4 0 "/Game/Geometry/Vehicles/Drone2/M_Metal_Drone2_Inst.M_Metal_Drone2_Inst"))
                    (`MaterialInstanceDynamic.SetVectorParameterValue` _returnvalue_52 "Base Color" (`self.RingColor`)))
                  (:`7`
                    (bind _returnvalue_53 (`PrimitiveComponent.CreateDynamicMaterialInstance` _carjet_4 0 "/Game/Geometry/Vehicles/Drone2/M_Alcantara_Drone2_Inst.M_Alcantara_Drone2_Inst"))
                    (`MaterialInstanceDynamic.SetVectorParameterValue` _returnvalue_53 "Base Color" (`self.RingColor`))
                    (`MaterialInstanceDynamic.SetVectorParameterValue` _returnvalue_53 "Rim Color" (`self.RingDetailColor`)))
                  (:`8`
                    (bind _returnvalue_54 (`PrimitiveComponent.CreateDynamicMaterialInstance` _carjet_4 0 "/Game/Geometry/Vehicles/Drone2/M_Fabric_ArchLiner_Drone2_Inst.M_Fabric_ArchLiner_Drone2_Inst"))
                    (`MaterialInstanceDynamic.SetVectorParameterValue` _returnvalue_54 "Base Color" (`self.RingColor`)))
                  (:`9`
                    (bind _returnvalue_55 (`PrimitiveComponent.CreateDynamicMaterialInstance` _carjet_4 0 "/Game/Geometry/Vehicles/Drone2/M_Leather_Drone2_Inst.M_Leather_Drone2_Inst"))
                    (`MaterialInstanceDynamic.SetVectorParameterValue` _returnvalue_55 "Base Color" (`self.RingColor`)))
                  (:`10`
                    (bind _returnvalue_56 (`PrimitiveComponent.CreateDynamicMaterialInstance` _carjet_4 0 "/Game/Geometry/Vehicles/Drone2/MI_MasterPerforated_Drone2_Inst.MI_MasterPerforated_Drone2_Inst"))
                    (`MaterialInstanceDynamic.SetVectorParameterValue` _returnvalue_56 "Base Color" (`self.RingColor`))
                    (`MaterialInstanceDynamic.SetVectorParameterValue` _returnvalue_56 "Perforation Color" (`self.RingDetailColor`)))))
              (:`then_2`
                (switch `int` RingMaterialNumber
                  (:`0`
                    (bind _returnvalue_57 (`PrimitiveComponent.CreateDynamicMaterialInstance` _carring 0 "/Game/Geometry/Vehicles/Drone2/M_Carpaint_Drone2_Inst.M_Carpaint_Drone2_Inst"))
                    (`MaterialInstanceDynamic.SetVectorParameterValue` _returnvalue_57 "Base Color" (`self.RingColor`))
                    (`MaterialInstanceDynamic.SetVectorParameterValue` _returnvalue_57 "Flake Color" (`self.RingDetailColor`))
                    (`MaterialInstanceDynamic.SetScalarParameterValue` _returnvalue_57 "Flake Brightness" (`self.RingDetailBrightness`)))
                  (:`1`
                    (bind _returnvalue_58 (`PrimitiveComponent.CreateDynamicMaterialInstance` _carring 0 "/Game/Geometry/Vehicles/Drone2/M_Plastic_Coated_Drone2_Inst.M_Plastic_Coated_Drone2_Inst"))
                    (`MaterialInstanceDynamic.SetVectorParameterValue` _returnvalue_58 "Base Color" (`self.RingColor`)))
                  (:`2`
                    (bind _returnvalue_59 (`PrimitiveComponent.CreateDynamicMaterialInstance` _carring 0 "/Game/Geometry/Vehicles/Drone2/M_Plastic_Matte_Drone2_Inst.M_Plastic_Matte_Drone2_Inst"))
                    (`MaterialInstanceDynamic.SetVectorParameterValue` _returnvalue_59 "Base Color" (`self.RingColor`)))
                  (:`3`
                    (bind _returnvalue_60 (`PrimitiveComponent.CreateDynamicMaterialInstance` _carring 0 "/Game/Geometry/Vehicles/Drone2/M_Plastic_Speckled_Drone2_Inst.M_Plastic_Speckled_Drone2_Inst"))
                    (`MaterialInstanceDynamic.SetVectorParameterValue` _returnvalue_60 "Base Color" (`self.RingColor`))
                    (`MaterialInstanceDynamic.SetVectorParameterValue` _returnvalue_60 "Flake Color" (`self.RingDetailColor`))
                    (`MaterialInstanceDynamic.SetScalarParameterValue` _returnvalue_60 "Flake Brightness" (`self.RingDetailBrightness`)))
                  (:`4`
                    (bind _returnvalue_61 (`PrimitiveComponent.CreateDynamicMaterialInstance` _carring 0 "/Game/Geometry/Vehicles/Drone2/M_CarbonFiber_Drone2_Inst.M_CarbonFiber_Drone2_Inst"))
                    (`MaterialInstanceDynamic.SetVectorParameterValue` _returnvalue_61 "Base Color" (`self.RingColor`)))
                  (:`5`
                    (bind _returnvalue_62 (`PrimitiveComponent.CreateDynamicMaterialInstance` _carring 0 "/Game/Geometry/Vehicles/Drone2/M_TireRubber_Drone2_Inst.M_TireRubber_Drone2_Inst"))
                    (`MaterialInstanceDynamic.SetVectorParameterValue` _returnvalue_62 "Base Color" (`self.RingColor`)))
                  (:`6`
                    (bind _returnvalue_63 (`PrimitiveComponent.CreateDynamicMaterialInstance` _carring 0 "/Game/Geometry/Vehicles/Drone2/M_Metal_Drone2_Inst.M_Metal_Drone2_Inst"))
                    (`MaterialInstanceDynamic.SetVectorParameterValue` _returnvalue_63 "Base Color" (`self.RingColor`)))
                  (:`7`
                    (bind _returnvalue_64 (`PrimitiveComponent.CreateDynamicMaterialInstance` _carring 0 "/Game/Geometry/Vehicles/Drone2/M_Alcantara_Drone2_Inst.M_Alcantara_Drone2_Inst"))
                    (`MaterialInstanceDynamic.SetVectorParameterValue` _returnvalue_64 "Base Color" (`self.RingColor`))
                    (`MaterialInstanceDynamic.SetVectorParameterValue` _returnvalue_64 "Rim Color" (`self.RingDetailColor`)))
                  (:`8`
                    (bind _returnvalue_65 (`PrimitiveComponent.CreateDynamicMaterialInstance` _carring 0 "/Game/Geometry/Vehicles/Drone2/M_Fabric_ArchLiner_Drone2_Inst.M_Fabric_ArchLiner_Drone2_Inst"))
                    (`MaterialInstanceDynamic.SetVectorParameterValue` _returnvalue_65 "Base Color" (`self.RingColor`)))
                  (:`9`
                    (bind _returnvalue_66 (`PrimitiveComponent.CreateDynamicMaterialInstance` _carring 0 "/Game/Geometry/Vehicles/Drone2/M_Leather_Drone2_Inst.M_Leather_Drone2_Inst"))
                    (`MaterialInstanceDynamic.SetVectorParameterValue` _returnvalue_66 "Base Color" (`self.RingColor`)))
                  (:`10`
                    (bind _returnvalue_67 (`PrimitiveComponent.CreateDynamicMaterialInstance` _carring 0 "/Game/Geometry/Vehicles/Drone2/MI_MasterPerforated_Drone2_Inst.MI_MasterPerforated_Drone2_Inst"))
                    (`MaterialInstanceDynamic.SetVectorParameterValue` _returnvalue_67 "Base Color" (`self.RingColor`))
                    (`MaterialInstanceDynamic.SetVectorParameterValue` _returnvalue_67 "Perforation Color" (`self.RingDetailColor`))))))
            (else
              ;[1 1 1] Drone3
              (if (== _returnvalue "drone3")
                (`|ExecutionSequence`
                  (:`then_0`
                    (switch `int` BodyMaterialNumber
                      (:`0`
                        (bind _returnvalue_68 (`PrimitiveComponent.CreateDynamicMaterialInstance` _car_4 0 "/Game/Geometry/Vehicles/Drone3/M_Carpaint_Drone3_Inst.M_Carpaint_Drone3_Inst"))
                        (`MaterialInstanceDynamic.SetVectorParameterValue` _returnvalue_68 "Base Color" (`self.BodyColor`))
                        (`MaterialInstanceDynamic.SetVectorParameterValue` _returnvalue_68 "Flake Color" (`self.BodyDetailColor`))
                        (`MaterialInstanceDynamic.SetScalarParameterValue` _returnvalue_68 "Flake Brightness" (`self.BodyDetailBrightness`)))
                      (:`1`
                        (bind _returnvalue_69 (`PrimitiveComponent.CreateDynamicMaterialInstance` _car_4 0 "/Game/Geometry/Vehicles/Drone3/M_Plastic_Coated_Drone3_Inst.M_Plastic_Coated_Drone3_Inst"))
                        (`MaterialInstanceDynamic.SetVectorParameterValue` _returnvalue_69 "Base Color" (`self.BodyColor`)))
                      (:`2`
                        (bind _returnvalue_70 (`PrimitiveComponent.CreateDynamicMaterialInstance` _car_4 0 "/Game/Geometry/Vehicles/Drone3/M_Plastic_Matte_Drone3_Inst.M_Plastic_Matte_Drone3_Inst"))
                        (`MaterialInstanceDynamic.SetVectorParameterValue` _returnvalue_70 "Base Color" (`self.BodyColor`)))
                      (:`3`
                        (bind _returnvalue_71 (`PrimitiveComponent.CreateDynamicMaterialInstance` _car_4 0 "/Game/Geometry/Vehicles/Drone3/M_Plastic_Speckled_Drone3_Inst.M_Plastic_Speckled_Drone3_Inst"))
                        (`MaterialInstanceDynamic.SetVectorParameterValue` _returnvalue_71 "Base Color" (`self.BodyColor`))
                        (`MaterialInstanceDynamic.SetVectorParameterValue` _returnvalue_71 "Flake Color" (`self.BodyDetailColor`))
                        (`MaterialInstanceDynamic.SetScalarParameterValue` _returnvalue_71 "Flake Brightness" (`self.BodyDetailBrightness`)))
                      (:`4`
                        (bind _returnvalue_72 (`PrimitiveComponent.CreateDynamicMaterialInstance` _car_4 0 "/Game/Geometry/Vehicles/Drone3/M_CarbonFiber_Drone3_Inst.M_CarbonFiber_Drone3_Inst"))
                        (`MaterialInstanceDynamic.SetVectorParameterValue` _returnvalue_72 "Base Color" (`self.BodyColor`)))
                      (:`5`
                        (bind _returnvalue_73 (`PrimitiveComponent.CreateDynamicMaterialInstance` _car_4 0 "/Game/Geometry/Vehicles/Drone3/M_TireRubber_Drone3_Inst.M_TireRubber_Drone3_Inst"))
                        (`MaterialInstanceDynamic.SetVectorParameterValue` _returnvalue_73 "Base Color" (`self.BodyColor`)))
                      (:`6`
                        (bind _returnvalue_74 (`PrimitiveComponent.CreateDynamicMaterialInstance` _car_4 0 "/Game/Geometry/Vehicles/Drone3/M_Metal_Drone3_Inst.M_Metal_Drone3_Inst"))
                        (`MaterialInstanceDynamic.SetVectorParameterValue` _returnvalue_74 "Base Color" (`self.BodyColor`)))
                      (:`7`
                        (bind _returnvalue_75 (`PrimitiveComponent.CreateDynamicMaterialInstance` _car_4 0 "/Game/Geometry/Vehicles/Drone3/M_Alcantara_Drone3_Inst.M_Alcantara_Drone3_Inst"))
                        (`MaterialInstanceDynamic.SetVectorParameterValue` _returnvalue_75 "Base Color" (`self.BodyColor`))
                        (`MaterialInstanceDynamic.SetVectorParameterValue` _returnvalue_75 "Rim Color" (`self.BodyDetailColor`)))
                      (:`8`
                        (bind _returnvalue_76 (`PrimitiveComponent.CreateDynamicMaterialInstance` _car_4 0 "/Game/Geometry/Vehicles/Drone3/M_Fabric_ArchLiner_Drone3_Inst.M_Fabric_ArchLiner_Drone3_Inst"))
                        (`MaterialInstanceDynamic.SetVectorParameterValue` _returnvalue_76 "Base Color" (`self.BodyColor`)))
                      (:`9`
                        (bind _returnvalue_77 (`PrimitiveComponent.CreateDynamicMaterialInstance` _car_4 0 "/Game/Geometry/Vehicles/Drone3/M_Leather_Drone3_Inst.M_Leather_Drone3_Inst"))
                        (`MaterialInstanceDynamic.SetVectorParameterValue` _returnvalue_77 "Base Color" (`self.BodyColor`)))
                      (:`10`
                        (bind _returnvalue_78 (`PrimitiveComponent.CreateDynamicMaterialInstance` _car_4 0 "/Game/Geometry/Vehicles/Drone3/MI_MasterPerforated_Drone3_Inst.MI_MasterPerforated_Drone3_Inst"))
                        (`MaterialInstanceDynamic.SetVectorParameterValue` _returnvalue_78 "Base Color" (`self.BodyColor`))
                        (`MaterialInstanceDynamic.SetVectorParameterValue` _returnvalue_78 "Perforation Color" (`self.BodyDetailColor`)))))
                  (:`then_1`
                    (switch `int` RingMaterialNumber
                      (:`0`
                        (bind _returnvalue_79 (`PrimitiveComponent.CreateDynamicMaterialInstance` _carjet_2 0 "/Game/Geometry/Vehicles/Drone3/M_Carpaint_Drone3_Inst.M_Carpaint_Drone3_Inst"))
                        (`MaterialInstanceDynamic.SetVectorParameterValue` _returnvalue_79 "Base Color" (`self.RingColor`))
                        (`MaterialInstanceDynamic.SetVectorParameterValue` _returnvalue_79 "Flake Color" (`self.RingDetailColor`))
                        (`MaterialInstanceDynamic.SetScalarParameterValue` _returnvalue_79 "Flake Brightness" (`self.RingDetailBrightness`)))
                      (:`1`
                        (bind _returnvalue_80 (`PrimitiveComponent.CreateDynamicMaterialInstance` _carjet_2 0 "/Game/Geometry/Vehicles/Drone3/M_Plastic_Coated_Drone3_Inst.M_Plastic_Coated_Drone3_Inst"))
                        (`MaterialInstanceDynamic.SetVectorParameterValue` _returnvalue_80 "Base Color" (`self.RingColor`)))
                      (:`2`
                        (bind _returnvalue_81 (`PrimitiveComponent.CreateDynamicMaterialInstance` _carjet_2 0 "/Game/Geometry/Vehicles/Drone3/M_Plastic_Matte_Drone3_Inst.M_Plastic_Matte_Drone3_Inst"))
                        (`MaterialInstanceDynamic.SetVectorParameterValue` _returnvalue_81 "Base Color" (`self.RingColor`)))
                      (:`3`
                        (bind _returnvalue_82 (`PrimitiveComponent.CreateDynamicMaterialInstance` _carjet_2 0 "/Game/Geometry/Vehicles/Drone3/M_Plastic_Speckled_Drone3_Inst.M_Plastic_Speckled_Drone3_Inst"))
                        (`MaterialInstanceDynamic.SetVectorParameterValue` _returnvalue_82 "Base Color" (`self.RingColor`))
                        (`MaterialInstanceDynamic.SetVectorParameterValue` _returnvalue_82 "Flake Color" (`self.RingDetailColor`))
                        (`MaterialInstanceDynamic.SetScalarParameterValue` _returnvalue_82 "Flake Brightness" (`self.RingDetailBrightness`)))
                      (:`4`
                        (bind _returnvalue_83 (`PrimitiveComponent.CreateDynamicMaterialInstance` _carjet_2 0 "/Game/Geometry/Vehicles/Drone3/M_CarbonFiber_Drone3_Inst.M_CarbonFiber_Drone3_Inst"))
                        (`MaterialInstanceDynamic.SetVectorParameterValue` _returnvalue_83 "Base Color" (`self.RingColor`)))
                      (:`5`
                        (bind _returnvalue_84 (`PrimitiveComponent.CreateDynamicMaterialInstance` _carjet_2 0 "/Game/Geometry/Vehicles/Drone3/M_TireRubber_Drone3_Inst.M_TireRubber_Drone3_Inst"))
                        (`MaterialInstanceDynamic.SetVectorParameterValue` _returnvalue_84 "Base Color" (`self.RingColor`)))
                      (:`6`
                        (bind _returnvalue_85 (`PrimitiveComponent.CreateDynamicMaterialInstance` _carjet_2 0 "/Game/Geometry/Vehicles/Drone3/M_Metal_Drone3_Inst.M_Metal_Drone3_Inst"))
                        (`MaterialInstanceDynamic.SetVectorParameterValue` _returnvalue_85 "Base Color" (`self.RingColor`)))
                      (:`7`
                        (bind _returnvalue_86 (`PrimitiveComponent.CreateDynamicMaterialInstance` _carjet_2 0 "/Game/Geometry/Vehicles/Drone3/M_Alcantara_Drone3_Inst.M_Alcantara_Drone3_Inst"))
                        (`MaterialInstanceDynamic.SetVectorParameterValue` _returnvalue_86 "Base Color" (`self.RingColor`))
                        (`MaterialInstanceDynamic.SetVectorParameterValue` _returnvalue_86 "Rim Color" (`self.RingDetailColor`)))
                      (:`8`
                        (bind _returnvalue_87 (`PrimitiveComponent.CreateDynamicMaterialInstance` _carjet_2 0 "/Game/Geometry/Vehicles/Drone3/M_Fabric_ArchLiner_Drone3_Inst.M_Fabric_ArchLiner_Drone3_Inst"))
                        (`MaterialInstanceDynamic.SetVectorParameterValue` _returnvalue_87 "Base Color" (`self.RingColor`)))
                      (:`9`
                        (bind _returnvalue_88 (`PrimitiveComponent.CreateDynamicMaterialInstance` _carjet_2 0 "/Game/Geometry/Vehicles/Drone3/M_Leather_Drone3_Inst.M_Leather_Drone3_Inst"))
                        (`MaterialInstanceDynamic.SetVectorParameterValue` _returnvalue_88 "Base Color" (`self.RingColor`)))
                      (:`10`
                        (bind _returnvalue_89 (`PrimitiveComponent.CreateDynamicMaterialInstance` _carjet_2 0 "/Game/Geometry/Vehicles/Drone3/MI_MasterPerforated_Drone3_Inst.MI_MasterPerforated_Drone3_Inst"))
                        (`MaterialInstanceDynamic.SetVectorParameterValue` _returnvalue_89 "Base Color" (`self.RingColor`))
                        (`MaterialInstanceDynamic.SetVectorParameterValue` _returnvalue_89 "Perforation Color" (`self.RingDetailColor`)))))
                  (:`then_2`
                    (switch `int` RingMaterialNumber
                      (:`0`
                        (bind _returnvalue_90 (`PrimitiveComponent.CreateDynamicMaterialInstance` _carring_3 0 "/Game/Geometry/Vehicles/Drone3/M_Carpaint_Drone3_Inst.M_Carpaint_Drone3_Inst"))
                        (`MaterialInstanceDynamic.SetVectorParameterValue` _returnvalue_90 "Base Color" (`self.RingColor`))
                        (`MaterialInstanceDynamic.SetVectorParameterValue` _returnvalue_90 "Flake Color" (`self.RingDetailColor`))
                        (`MaterialInstanceDynamic.SetScalarParameterValue` _returnvalue_90 "Flake Brightness" (`self.RingDetailBrightness`)))
                      (:`1`
                        (bind _returnvalue_91 (`PrimitiveComponent.CreateDynamicMaterialInstance` _carring_3 0 "/Game/Geometry/Vehicles/Drone3/M_Plastic_Coated_Drone3_Inst.M_Plastic_Coated_Drone3_Inst"))
                        (`MaterialInstanceDynamic.SetVectorParameterValue` _returnvalue_91 "Base Color" (`self.RingColor`)))
                      (:`2`
                        (bind _returnvalue_92 (`PrimitiveComponent.CreateDynamicMaterialInstance` _carring_3 0 "/Game/Geometry/Vehicles/Drone3/M_Plastic_Matte_Drone3_Inst.M_Plastic_Matte_Drone3_Inst"))
                        (`MaterialInstanceDynamic.SetVectorParameterValue` _returnvalue_92 "Base Color" (`self.RingColor`)))
                      (:`3`
                        (bind _returnvalue_93 (`PrimitiveComponent.CreateDynamicMaterialInstance` _carring_3 0 "/Game/Geometry/Vehicles/Drone3/M_Plastic_Speckled_Drone3_Inst.M_Plastic_Speckled_Drone3_Inst"))
                        (`MaterialInstanceDynamic.SetVectorParameterValue` _returnvalue_93 "Base Color" (`self.RingColor`))
                        (`MaterialInstanceDynamic.SetVectorParameterValue` _returnvalue_93 "Flake Color" (`self.RingDetailColor`))
                        (`MaterialInstanceDynamic.SetScalarParameterValue` _returnvalue_93 "Flake Brightness" (`self.RingDetailBrightness`)))
                      (:`4`
                        (bind _returnvalue_94 (`PrimitiveComponent.CreateDynamicMaterialInstance` _carring_3 0 "/Game/Geometry/Vehicles/Drone3/M_CarbonFiber_Drone3_Inst.M_CarbonFiber_Drone3_Inst"))
                        (`MaterialInstanceDynamic.SetVectorParameterValue` _returnvalue_94 "Base Color" (`self.RingColor`)))
                      (:`5`
                        (bind _returnvalue_95 (`PrimitiveComponent.CreateDynamicMaterialInstance` _carring_3 0 "/Game/Geometry/Vehicles/Drone3/M_TireRubber_Drone3_Inst.M_TireRubber_Drone3_Inst"))
                        (`MaterialInstanceDynamic.SetVectorParameterValue` _returnvalue_95 "Base Color" (`self.RingColor`)))
                      (:`6`
                        (bind _returnvalue_96 (`PrimitiveComponent.CreateDynamicMaterialInstance` _carring_3 0 "/Game/Geometry/Vehicles/Drone3/M_Metal_Drone3_Inst.M_Metal_Drone3_Inst"))
                        (`MaterialInstanceDynamic.SetVectorParameterValue` _returnvalue_96 "Base Color" (`self.RingColor`)))
                      (:`7`
                        (bind _returnvalue_97 (`PrimitiveComponent.CreateDynamicMaterialInstance` _carring_3 0 "/Game/Geometry/Vehicles/Drone3/M_Alcantara_Drone3_Inst.M_Alcantara_Drone3_Inst"))
                        (`MaterialInstanceDynamic.SetVectorParameterValue` _returnvalue_97 "Base Color" (`self.RingColor`))
                        (`MaterialInstanceDynamic.SetVectorParameterValue` _returnvalue_97 "Rim Color" (`self.RingDetailColor`)))
                      (:`8`
                        (bind _returnvalue_98 (`PrimitiveComponent.CreateDynamicMaterialInstance` _carring_3 0 "/Game/Geometry/Vehicles/Drone3/M_Fabric_ArchLiner_Drone3_Inst.M_Fabric_ArchLiner_Drone3_Inst"))
                        (`MaterialInstanceDynamic.SetVectorParameterValue` _returnvalue_98 "Base Color" (`self.RingColor`)))
                      (:`9`
                        (bind _returnvalue_99 (`PrimitiveComponent.CreateDynamicMaterialInstance` _carring_3 0 "/Game/Geometry/Vehicles/Drone3/M_Leather_Drone3_Inst.M_Leather_Drone3_Inst"))
                        (`MaterialInstanceDynamic.SetVectorParameterValue` _returnvalue_99 "Base Color" (`self.RingColor`)))
                      (:`10`
                        (bind _returnvalue_100 (`PrimitiveComponent.CreateDynamicMaterialInstance` _carring_3 0 "/Game/Geometry/Vehicles/Drone3/MI_MasterPerforated_Drone3_Inst.MI_MasterPerforated_Drone3_Inst"))
                        (`MaterialInstanceDynamic.SetVectorParameterValue` _returnvalue_100 "Base Color" (`self.RingColor`))
                        (`MaterialInstanceDynamic.SetVectorParameterValue` _returnvalue_100 "Perforation Color" (`self.RingDetailColor`))))))))))))))

(fn `JetAndRingRotation`
  (bind _returnvalue (`KismetMathLibrary.MakeRotator` 0.0 0.0 1.0))
  (`SceneComponent.K2_AddLocalRotation` (`self.CarJet`) _returnvalue false false)
  (`SceneComponent.K2_AddLocalRotation` (`self.CarRing`) (`KismetMathLibrary.NegateRotator` _returnvalue) false false))

(fn `ResetRotation`
  (`self.K2_SetActorRelativeRotation` (struct)))

(fn `UserConstructionScript`)