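; Hover component for a vehicle, apparently the bumper car, that pushes a physics-simulated mesh, supplied through InitComponent, away from surfaces beneath it.
; Each tick it traces down its local axis and applies force along the hit normal at its own location, lerped from HoverForce toward a fixed value by hit distance.
; Hits set configured linear and angular damping; misses set only a fixed linear damping.
; The bumper car lookup for the trace's ignore list is disconnected.
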(event Custom|InitComponent
  (params (MeshComponent :type Static%20Mesh%20Component%20Object%20Reference))
  (bind _output_get (Variables|Default|SetParentComponent MeshComponent))
  (Physics|SetSimulatePhysics _output_get true))

(event EventTick
  (params (DeltaSeconds :type Float%20%28single-precision%29))
  (bind _returnvalue (Transformation|GetWorldLocation))
  (bind _parentcomponent (Variables|Default|GetParentComponent))
  (bind (_outhit _returnvalue_2) (Collision|LineTraceByChannel _returnvalue (+ _returnvalue (* (Math|Vector|GetUpVector) (* (Variables|Default|GetTraceLength) -1.0))) "TraceTypeQuery1" false (Utilities|Array|MakeArray (stale _asbumper_car)) "None"))
  (if _returnvalue_2
    (Variables|Default|SetHittingSomething true)
    (Variables|Default|SetTEST 1.0)
    (Class|PrimitiveComponent|AddForceatLocation _parentcomponent (* (.ImpactNormal (Collision|BreakHitResult _outhit)) (* (Math|Float|Lerp (Variables|Default|GetHoverForce) 5e+04 (/ (Math|Vector|VectorLength (- (.Location (Collision|BreakHitResult _outhit)) (Transformation|GetWorldLocation))) (Variables|Default|GetTraceLength))) (Variables|Default|GetTEST))) (Transformation|GetWorldLocation) "None")
    (Class|PrimitiveComponent|SetLinearDamping _parentcomponent (Variables|Default|GetLinearDamping))
    (Class|PrimitiveComponent|SetAngularDamping _parentcomponent (Variables|Default|GetAngularDamping))
    (else
      (Variables|Default|SetHittingSomething false)
      (Class|PrimitiveComponent|SetLinearDamping (Variables|Default|GetParentComponent) 0.5))))