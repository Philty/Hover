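; CarPreviewer is an actor that displays a selected drone-style vehicle, registering itself with MyGameInstance on BeginPlay.
; Every Tick it polls the first CarMesh entry in the game instance and passes it to ChangeVehicleMesh.
; That function switches between three drones, swapping body, jet and ring meshes, and sets a paint material for the first two only.
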(event `self.ReceiveBeginPlay`
  ;[1 1 1] Give MyGameInstance a reference to the previewer
  (bind _asmy_game_instance (cast `/Game/Blueprints/MyGameInstance` (`GameplayStatics.GetGameInstance`)))
  (set `/Game/Blueprints/MyGameInstance.CarPreviewerReference` self _asmy_game_instance))

(event `self.ReceiveTick`
  (params (DeltaSeconds :type "Float (single-precision)"))
  (bind _asmy_game_instance (cast `/Game/Blueprints/MyGameInstance` (`GameplayStatics.GetGameInstance`)))
  (`self.ChangeVehicleMesh` (`KismetArrayLibrary.Array_Get` (`/Game/Blueprints/MyGameInstance.CarMesh` _asmy_game_instance))))

(fn `ChangeVehicleMesh`
  (params (StaticMeshInteger :type Integer))
  (bind _car (`self.Car`))
  (switch `int` StaticMeshInteger
    (:`0`
      (`StaticMeshComponent.SetStaticMesh` _car "/Game/Geometry/Vehicles/Drone1/Drone1.Drone1")
      (`StaticMeshComponent.SetStaticMesh` (`self.CarJet`) "/Game/Geometry/Vehicles/Drone1/Drone1Jet.Drone1Jet")
      (`StaticMeshComponent.SetStaticMesh` (`self.CarRing`) "/Game/Geometry/Vehicles/Drone1/Drone1Ring.Drone1Ring")
      (`PrimitiveComponent.SetMaterial` _car 0 "/Game/Materials/CarPaint/MI_CarPaint_13_Green.MI_CarPaint_13_Green"))
    (:`1`
      (`StaticMeshComponent.SetStaticMesh` _car "/Game/Geometry/Vehicles/Drone2/Drone2.Drone2")
      (`StaticMeshComponent.SetStaticMesh` (`self.CarJet`) "/Game/Geometry/Vehicles/Drone2/Drone2Jet.Drone2Jet")
      (`StaticMeshComponent.SetStaticMesh` (`self.CarRing`) "/Game/Geometry/Vehicles/Drone2/Drone2Ring.Drone2Ring")
      (`PrimitiveComponent.SetMaterial` _car 0 "/Game/Materials/CarPaint/MI_CarPaint_02_DarkRedBlack.MI_CarPaint_02_DarkRedBlack"))
    (:`2`
      (`StaticMeshComponent.SetStaticMesh` _car "/Game/Geometry/Vehicles/Drone3/Drone3.Drone3")
      (`StaticMeshComponent.SetStaticMesh` (`self.CarJet`) "/Game/Geometry/Vehicles/Drone3/Drone3Jet.Drone3Jet")
      (`StaticMeshComponent.SetStaticMesh` (`self.CarRing`) "/Game/Geometry/Vehicles/Drone3/Drone3Ring.Drone3Ring"))))

(fn `UserConstructionScript`)