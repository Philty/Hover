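; Pickup actor that makes the BumperCar overlapping it untaggable for eight seconds.
; On overlap it turns off its collision and visibility, clears the car's CanBeTagged flag, activates the car's PPickup component and tells MyGameInstance no pickup is in the level.
; The hidden actor stays alive through a Delay to restore CanBeTagged, then destroys itself.
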(event `self.ReceiveActorBeginOverlap`
  (params (OtherActor :type "Actor Object Reference"))
  (bind _asbumper_car (cast `/Game/Blueprints/Vehicles/BumperCar` OtherActor))
  (`self.SetActorEnableCollision` false)
  (`self.SetActorHiddenInGame` true)
  (set `/Game/Blueprints/Vehicles/BumperCar.CanBeTagged` false _asbumper_car)
  (`ActorComponent.Activate` (`/Game/Blueprints/Vehicles/BumperCar.P_Pickup` _asbumper_car) false)
  (bind _asmy_game_instance (cast `/Game/Blueprints/MyGameInstance` (`GameplayStatics.GetGameInstance`)))
  (set `/Game/Blueprints/MyGameInstance.IsThereAPickupInLevel` false _asmy_game_instance)
  (`KismetSystemLibrary.Delay` 8.0)
  (set `/Game/Blueprints/Vehicles/BumperCar.CanBeTagged` true _asbumper_car)
  (`self.K2_DestroyActor`))

(fn `UserConstructionScript`)