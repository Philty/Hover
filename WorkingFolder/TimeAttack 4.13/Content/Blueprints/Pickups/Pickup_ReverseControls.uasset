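; Pickup that temporarily reverses the controls of the bumper car that overlaps it.
; On overlap it sets the car's reversed flag, negates its moving and turning speeds and activates its pickup component.
; It also clears the game instance's pickup-in-level flag and hides itself, leaving collision untouched.
; After an eight-second delay it negates the speeds again, clears the reversed flag and destroys itself.
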(event `self.ReceiveActorBeginOverlap`
  (params (OtherActor :type "Actor Object Reference"))
  (bind _asbumper_car (cast `/Game/Blueprints/Vehicles/BumperCar` OtherActor))
  (set `/Game/Blueprints/Vehicles/BumperCar.ReversedControls` true _asbumper_car)
  (set `/Game/Blueprints/Vehicles/BumperCar.MovingSpeed` (* -1.0 (`/Game/Blueprints/Vehicles/BumperCar.MovingSpeed` _asbumper_car)) _asbumper_car)
  (set `/Game/Blueprints/Vehicles/BumperCar.TurningSpeed` (* -1.0 (`/Game/Blueprints/Vehicles/BumperCar.TurningSpeed` _asbumper_car)) _asbumper_car)
  (`ActorComponent.Activate` (`/Game/Blueprints/Vehicles/BumperCar.P_Pickup` _asbumper_car) false)
  (bind _asmy_game_instance (cast `/Game/Blueprints/MyGameInstance` (`GameplayStatics.GetGameInstance`)))
  (set `/Game/Blueprints/MyGameInstance.IsThereAPickupInLevel` false _asmy_game_instance)
  (`self.SetActorHiddenInGame` true)
  (`KismetSystemLibrary.Delay` 8.0)
  (set `/Game/Blueprints/Vehicles/BumperCar.ReversedControls` false _asbumper_car)
  (set `/Game/Blueprints/Vehicles/BumperCar.MovingSpeed` (* -1.0 (`/Game/Blueprints/Vehicles/BumperCar.MovingSpeed` _asbumper_car)) _asbumper_car)
  (set `/Game/Blueprints/Vehicles/BumperCar.TurningSpeed` (* -1.0 (`/Game/Blueprints/Vehicles/BumperCar.TurningSpeed` _asbumper_car)) _asbumper_car)
  (`self.K2_DestroyActor`))

(fn `UserConstructionScript`)