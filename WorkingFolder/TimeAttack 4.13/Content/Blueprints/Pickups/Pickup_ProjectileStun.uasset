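; Pickup actor that grants a bumper car the stun projectile weapon in the bumper-car game.
; On overlap with a BumperCar it enables shooting, sets the ammo type to BulletStun and activates the car's PPickup component.
; It then clears the GameInstance's pickup-in-level flag and destroys itself.
; Tick spins the actor in yaw by a fixed step per frame, independent of delta time.
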(event `self.ReceiveBeginPlay`)

(event `self.ReceiveActorBeginOverlap`
  (params (OtherActor :type "Actor Object Reference"))
  (bind _asbumper_car (cast `/Game/Blueprints/Vehicles/BumperCar` OtherActor))
  (set `/Game/Blueprints/Vehicles/BumperCar.CanShoot` true _asbumper_car)
  (set `/Game/Blueprints/Vehicles/BumperCar.AmmoType` "/Game/Blueprints/Projectiles/BulletStun.BulletStun_C" _asbumper_car)
  (`ActorComponent.Activate` (`/Game/Blueprints/Vehicles/BumperCar.P_Pickup` _asbumper_car) false)
  (bind _asmy_game_instance (cast `/Game/Blueprints/MyGameInstance` (`GameplayStatics.GetGameInstance`)))
  (set `/Game/Blueprints/MyGameInstance.IsThereAPickupInLevel` false _asmy_game_instance)
  (`self.K2_DestroyActor`))

(event `self.ReceiveTick`
  (params (DeltaSeconds :type "Float (single-precision)"))
  (`self.K2_SetActorTransform` (`KismetMathLibrary.MakeTransform` (`self.K2_GetActorLocation`) (`KismetMathLibrary.MakeRotator` (.roll (`self.K2_GetActorRotation`)) (.pitch (`self.K2_GetActorRotation`)) (+ (.yaw (`self.K2_GetActorRotation`)) 1.0)) (`self.GetActorScale3D`))))

(fn `UserConstructionScript`)