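; Bumper car pickup that temporarily slows every player except the one who drives over it.
; On overlap it loops through player pawns by index, halving the other cars' moving and turning speeds, and activates the collector's pickup effect.
; It clears the game instance's pickup-in-level flag and hides itself, leaving collision untouched.
; After a fixed delay it doubles those speeds back and destroys itself.
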(event `self.ReceiveBeginPlay`
  (bind _asmy_game_instance (cast `/Game/Blueprints/MyGameInstance` (`GameplayStatics.GetGameInstance`)))
  (set `self.LastPlayerIndex` (- (`/Game/Blueprints/MyGameInstance.IntNumberOfPlayers` _asmy_game_instance) 1)))

(event `self.ReceiveActorBeginOverlap`
  (params (OtherActor :type "Actor Object Reference"))
  ;[1 1 1] Cycling through all bumpercars and adjusting speed on the ones that didn't overlap this pickup
  (bind _asbumper_car (cast `/Game/Blueprints/Vehicles/BumperCar` OtherActor))
  (set `self.OverlappedBumperCarIndex` (`/Game/Blueprints/Vehicles/BumperCar.PlayerIndexCache` _asbumper_car))
  (for _index (range (+ (`self.LastPlayerIndex`) 1))
    (if (!= _index (`self.OverlappedBumperCarIndex`))
      (bind _asbumper_car_2 (cast `/Game/Blueprints/Vehicles/BumperCar` (`GameplayStatics.GetPlayerPawn` _index)))
      (set `/Game/Blueprints/Vehicles/BumperCar.MovingSpeed` (/ (`/Game/Blueprints/Vehicles/BumperCar.MovingSpeed` _asbumper_car_2) 2.0) _asbumper_car_2)
      (set `/Game/Blueprints/Vehicles/BumperCar.TurningSpeed` (/ (`/Game/Blueprints/Vehicles/BumperCar.TurningSpeed` _asbumper_car_2) 2.0) _asbumper_car_2)))
  (`ActorComponent.Activate` (`/Game/Blueprints/Vehicles/BumperCar.P_Pickup` _asbumper_car) false)
  (bind _asmy_game_instance (cast `/Game/Blueprints/MyGameInstance` (`GameplayStatics.GetGameInstance`)))
  (set `/Game/Blueprints/MyGameInstance.IsThereAPickupInLevel` false _asmy_game_instance)
  (`self.SetActorHiddenInGame` true)
  (`KismetSystemLibrary.Delay` 8.0)
  (for _index_2 (range (+ (`self.LastPlayerIndex`) 1))
    (if (!= _index_2 (`self.OverlappedBumperCarIndex`))
      (bind _asbumper_car_3 (cast `/Game/Blueprints/Vehicles/BumperCar` (`GameplayStatics.GetPlayerPawn` _index_2)))
      (set `/Game/Blueprints/Vehicles/BumperCar.MovingSpeed` (* (`/Game/Blueprints/Vehicles/BumperCar.MovingSpeed` _asbumper_car_3) 2.0) _asbumper_car_3)
      (set `/Game/Blueprints/Vehicles/BumperCar.TurningSpeed` (* (`/Game/Blueprints/Vehicles/BumperCar.TurningSpeed` _asbumper_car_3) 2.0) _asbumper_car_3)))
  (`self.K2_DestroyActor`))

(fn `UserConstructionScript`)